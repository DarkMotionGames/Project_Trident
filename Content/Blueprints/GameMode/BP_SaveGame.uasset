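; SaveGame object that stores and restores the player's quest log and per-quest progress.
; SaveQuestLog copies the active and completed quest lists, while SaveQuestDetails records each quest's stage and objective progress in a map keyed by quest ID.
; LoadQuest re-adds each active quest to the given QuestLog, applies its saved stage and progress, then restores both lists.
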(fn SaveQuestDetails
  (params (QuestObject :type BP%20Quest%20Base%20Object%20Reference))
  (Utilities|Map|Add (Variables|Default|GetQuestProgress) (Variables|/Game/QuestSystem/Blueprint/BP_QuestBase.BP_QuestBase_C|GetQuestID QuestObject) (Utilities|Struct|MakeF_SaveData (Variables|/Game/QuestSystem/Blueprint/BP_QuestBase.BP_QuestBase_C|GetCurrentObjectiveProgress QuestObject) (Variables|/Game/QuestSystem/Blueprint/BP_QuestBase.BP_QuestBase_C|GetCurrentStage QuestObject))))

(fn LoadQuest
  (params (QuestLog :type BAC%20Quest%20Log%20Object%20Reference))
  (for _array_element (Variables|Default|GetCurrentActiveQuest)
    (bind _returnvalue (Default|AddNewQuest QuestLog _array_element))
    (Variables|/Game/QuestSystem/Blueprint/BP_QuestBase.BP_QuestBase_C|SetCurrentStage _returnvalue (.CurrenStage (Utilities|Struct|BreakF_SaveData (.Value (Utilities|Map|Find (Variables|Default|GetQuestProgress) _array_element)))))
    (Variables|/Game/QuestSystem/Blueprint/BP_QuestBase.BP_QuestBase_C|SetCurrentObjectiveProgress _returnvalue (.Progress (Utilities|Struct|BreakF_SaveData (.Value (Utilities|Map|Find (Variables|Default|GetQuestProgress) _array_element))))))
  (Variables|/Game/QuestSystem/Blueprint/BAC_QuestLog.BAC_QuestLog_C|SetCurrentActiveQuest QuestLog (Variables|Default|GetCurrentActiveQuest))
  (Variables|/Game/QuestSystem/Blueprint/BAC_QuestLog.BAC_QuestLog_C|SetCompletedQuest QuestLog (Variables|Default|GetCompletedQuest)))

(fn SaveQuestLog
  (params (QuestLog :type BAC%20Quest%20Log%20Object%20Reference))
  (Variables|Default|SetCurrentActiveQuest (Variables|/Game/QuestSystem/Blueprint/BAC_QuestLog.BAC_QuestLog_C|GetCurrentActiveQuest QuestLog))
  (Variables|Default|SetCompletedQuest (Variables|/Game/QuestSystem/Blueprint/BAC_QuestLog.BAC_QuestLog_C|GetCompletedQuest QuestLog)))