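; BP_Weapon is a weapon actor that adds one "weapon" item to the player's inventory on overlap and can apply Chaos destruction fields.
; CreateFields applies a linear-falloff external cluster strain and a radial linear force at a given location to break and scatter destructibles.
; Overlap casts to BP_Player and calls its BACInventory component, without removing the actor.
; InteractWith returns the weapon's ObjectiveId.
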(event EventBeginPlay)

(event Collision|EventActorBeginOverlap
  (params (OtherActor :type Actor%20Object%20Reference))
  (bind _asbp_player (Utilities|Casting|CastToBP_Player OtherActor))
  (Default|AddtoInventory (Variables|/Game/Blueprints/Player/BP_Player.BP_Player_C|GetBAC_Inventory _asbp_player) "weapon" 1))

(event EventCreateFields
  (params (FieldLocation :type Vector%20%28by%20ref%29 :default "0, 0, 0"))
  (bind _fieldsystem (Variables|Default|GetFieldSystem))
  (bind _fieldsystemmetadatafilter (Variables|Default|GetFieldSystemMetaDataFilter))
  (Class|FieldSystemComponent|ApplyPhysicsField _fieldsystem true "Field_ExternalClusterStrain" _fieldsystemmetadatafilter (Field|SetRadialFalloff (Variables|Default|GetRadialFalloff) 1e+06 0.8 1.0 0.0 2e+02 FieldLocation "Field_Falloff_Linear"))
  (Class|FieldSystemComponent|ApplyPhysicsField _fieldsystem true "Field_LinearForce" _fieldsystemmetadatafilter (Field|SetRadialVector (Variables|Default|GetRadialVector) 1.5e+07 FieldLocation)))

(fn ConstructionScript)

(fn Interactwith
  (return (Variables|Default|GetObjective%20Id)))