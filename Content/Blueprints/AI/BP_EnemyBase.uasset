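; BP_EnemyBase is the base enemy Blueprint, handling hit reactions, attack motion warping and death rewards.
; Tick feeds translation and rotation warp targets to Motion Warping while a combat target is valid, and GetHit defers to the parent.
; A looping timer started at BeginPlay polls health; once it hits zero, it reports objective progress to the player, awards experience and clears itself.
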(event Custom|OnDeath
  ;[1 1 1] OnDeath Spawn Widget
  (if (<= (Variables|/Script/Project_Trident.AttributeComponent|GetHealth (Variables|Default|GetAttributes)) 0.0)
    (bind _asbp_player (Utilities|Casting|CastToBP_Player (Game|GetPlayerCharacter 0)))
    (Default|CallOnObjectiveIdCalled _asbp_player (Variables|Default|GetObjectiveId) 1)
    (Default|AddExpPoints (CallFunction|GetMainPlayer) 75)
    (Utilities|Time|ClearandInvalidateTimerbyHandle (Variables|Default|GetDeathTimerReset))))

(event EventBeginPlay
  (bind _returnvalue (Utilities|Time|SetTimerbyEvent (delegate Custom|OnDeath) 1.0 true))
  (Variables|Default|SetDeathTimerReset _returnvalue))

(event EventTick
  (params (DeltaSeconds :type Float%20%28single-precision%29))
  (bind _motionwarping (Variables|Default|GetMotionWarping))
  (Variables|Default|GetCombatTarget
    (:then
      (bind _returnvalue (Class|BaseCharacter|GetTranslationWarpTarget))
      (Class|MotionWarpingComponent|AddorUpdateWarpTargetfromLocation _motionwarping "TrasnslationTarget" _returnvalue)
      (bind _returnvalue_2 (Class|BaseCharacter|GetRotationWarpTarget))
      (Class|MotionWarpingComponent|AddorUpdateWarpTargetfromLocation _motionwarping "RotationTarget" _returnvalue_2))
    (:else)))

(event EventGetHit
  (params (ImpactPoint :type Vector%20%28by%20ref%29 :default "0, 0, 0") (Hitter :type Actor%20Object%20Reference))
  (|CallParentFunction ImpactPoint Hitter))

(fn ConstructionScript)