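; BP_OldLady is an NPC the player can talk to, identifying itself as "oldlady" through InteractWith.
; Overlapping its box shows a text prompt, hidden again when the player leaves.
; Each Talk event increments an index and replaces the dialogue widget with the matching line from the Dialogue array.
; Tick removes the widget at a hardcoded final index, while logic to re-enable player input is left unconnected.
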(event OnComponentBeginOverlap(Box)
  (params (OverlappedComponent :type Primitive%20Component%20Object%20Reference) (OtherActor :type Actor%20Object%20Reference) (OtherComp :type Primitive%20Component%20Object%20Reference) (OtherBodyIndex :type Integer) (bFromSweep :type Boolean) (SweepResult :type Hit%20Result%20Structure%20%28by%20ref%29))
  (Utilities|Casting|CastToBP_Player OtherActor)
  (Development|SetHiddeninGame (Variables|Default|GetTextRender) false false))

(event OnComponentEndOverlap(Box)
  (params (OverlappedComponent :type Primitive%20Component%20Object%20Reference) (OtherActor :type Actor%20Object%20Reference) (OtherComp :type Primitive%20Component%20Object%20Reference) (OtherBodyIndex :type Integer))
  (Utilities|Casting|CastToBP_Player OtherActor)
  (Development|SetHiddeninGame (Variables|Default|GetTextRender) true false))

(event EventTalk
  (Math|Integer|IncrementInt (Variables|Default|GetTalkIndex)
    (:%20%20
      (if (<= (Variables|Default|GetTalkIndex) (Utilities|Array|Length (Variables|Default|GetDialogue)))
        (Widget|RemovefromParent (Variables|Default|GetW_Dialogue))
        (bind _returnvalue (UserInterface|CreateWidget "/Game/QuestSystem/Widgets/W_Dialogue.W_Dialogue_C" (Game|GetPlayerController 0)))
        (bind _output_get (Variables|Default|SetW_Dialogue _returnvalue))
        (UserInterface|Viewport|AddtoViewport _output_get 0)
        (Rendering|Components|TextRender|SetText (Variables|/Game/QuestSystem/Widgets/W_Dialogue.W_Dialogue_C|GetT_Dialogue (Variables|Default|GetW_Dialogue)) (Utilities|Text|ToText(String) (Utilities|Array|Get(acopy) (Variables|Default|GetDialogue) (Variables|Default|GetTalkIndex))))))))

(event EventGetHit
  (params (ImpactPoint :type Vector%20%28by%20ref%29 :default "0, 0, 0") (Hitter :type Actor%20Object%20Reference))
  (|CallParentFunction ImpactPoint Hitter))

(event EventTick
  (params (DeltaSeconds :type Float%20%28single-precision%29))
  (if (== (Variables|Default|GetTalkIndex) 8)
    (Widget|RemovefromParent (Variables|Default|GetW_Dialogue))))

(fn ConstructionScript)

(fn Interactwith
  (return "oldlady"))