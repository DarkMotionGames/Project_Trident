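; Player Blueprint that handles experience and leveling, interaction, death detection, and the pause, journal and retry widgets.
; BeginPlay caches the HUD, starts a looping health check that shows the retry screen, and loads quests from the GameInstance.
; AddExpPoints loops level-ups with growing thresholds and updates the HUD; F is a debug trigger.
; Interact sphere-traces forward for BPI_Interact actors, reporting objective IDs and triggering BPI_Dialogue talk.
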(event Custom|OnLevelUp
  ;[1 1 1] LevelUp!
  (Variables|Default|SetCurrentExp (- (Variables|Default|GetCurrentExp) (Variables|Default|GetExpForNextLevel)))
  (Variables|Default|SetExpForNextLevel (Math|Float|Truncate (* (Variables|Default|GetExpForNextLevel) (Variables|Default|GetNextExpMultiplier))))
  (Math|Integer|IncrementInt (Variables|Default|GetCurrentLevel)
    (:%20%20
      (ExpSystem|UpdateLevel)
      (Components|Activation|Activate (Variables|Default|GetLevelUpEffect) false))))

(event Custom|OnDeath
  ;[1 1 1] OnDeath Spawn Widget
  (if (<= (Variables|/Script/Project_Trident.AttributeComponent|GetHealth (Variables|Default|GetAttributes)) 1.0)
    (Utilities|FlowControl|DoOnce false
      (:Completed
        (bind _returnvalue (UserInterface|CreateWidget "/Game/UI/Menu/W_Retry.W_Retry_C"))
        (UserInterface|Viewport|AddtoViewport _returnvalue 0)
        (Utilities|Time|ClearandInvalidateTimerbyHandle (Variables|Default|GetDeathTimerReset))))))

(event Input|EnhancedActionEvents|EnhancedInputActionIA_Pause
  (params (ActionValue :type Boolean) (ElapsedSeconds :type Float%20%28double-precision%29) (TriggeredSeconds :type Float%20%28double-precision%29) (InputAction :type Input%20Action%20Object%20Reference :default "/Game/Blueprints/Player/Input/Actions/IA_Pause.IA_Pause"))
  ;[1 1 1] Pause Menu
  (:Started
    (bind _returnvalue (UserInterface|CreateWidget "/Game/UI/Menu/W_Pause.W_Pause_C"))
    (bind _output_get (Variables|Default|SetPause _returnvalue))
    (UserInterface|Viewport|AddtoViewport _output_get 0)))

(event Input|EnhancedActionEvents|EnhancedInputActionIA_Interact
  (params (ActionValue :type Boolean) (ElapsedSeconds :type Float%20%28double-precision%29) (TriggeredSeconds :type Float%20%28double-precision%29) (InputAction :type Input%20Action%20Object%20Reference :default "/Game/Blueprints/Player/Input/Actions/IA_Interact.IA_Interact"))
  ;[1 1 1] Interact
  (:Started
    (Utilities|FlowControl|Sequence
      (:then_0
        (CallFunction|InteractionTrace)
        (bind _lookatactor (Variables|Default|GetLookAtActor)
          (:then
            (bind _objectiveid (Class|BPIInteract|Interactwith(Message) _lookatactor))
            (Default|CallOnObjectiveIdCalled _objectiveid 1))
          (:else)))
      (:then_1
        (if (Utilities|DoesObjectImplementInterface (Variables|Default|GetLookAtActor) "/Game/QuestSystem/Blueprint/Dialogue/BPI_Dialogue.BPI_Dialogue_C")
          (Class|BPIDialogue|Talk(Message) _lookatactor))))))

(event Input|EnhancedActionEvents|EnhancedInputActionIA_Journal
  (params (ActionValue :type Boolean) (ElapsedSeconds :type Float%20%28double-precision%29) (TriggeredSeconds :type Float%20%28double-precision%29) (InputAction :type Input%20Action%20Object%20Reference :default "/Game/Blueprints/Player/Input/Actions/IA_Journal.IA_Journal"))
  (:Started
    (bind _returnvalue (UserInterface|CreateWidget "/Game/QuestSystem/Widgets/W_QuestLog.W_QuestLog_C"))
    (UserInterface|Viewport|AddtoViewport _returnvalue 0)))

(event EventBeginPlay
  (Utilities|FlowControl|Sequence
    (:then_0
      (Utilities|FlowControl|Delay 0.1)
      ;[1 1 1] HUD Reference
      (bind _foundwidgets (Widget|GetAllWidgetsOfClass "/Game/UI/WB_HUD.WB_HUD_C" true))
      (Variables|Default|SetHUD (Utilities|Array|Get(acopy) _foundwidgets))
      (ExpSystem|UpdateLevel)
      (ExpSystem|UpdateExp))
    (:then_1
      (bind _returnvalue (Utilities|Time|SetTimerbyEvent (delegate Custom|OnDeath) 1.0 true))
      (Variables|Default|SetDeathTimerReset _returnvalue))
    (:then_2
      ;[1 1 1] Load Game
      (bind _asbp_game_instance (Utilities|Casting|CastToBP_GameInstance (Game|GetGameInstance)))
      (Default|LoadQuest (Variables|/Game/Blueprints/GameMode/BP_GameInstance.BP_GameInstance_C|GetSaveData _asbp_game_instance) (Variables|Default|GetBAC_QuestLog)))))

(event Input|KeyboardEvents|F
  (params (Key :type Key%20Structure))
  ;[1 0 0] DebugOnly
  (:Pressed
    (ExpSystem|AddExpPoints 50)))

(fn ConstructionScript)

(fn UpdateExp
  (bind _hud (Variables|Default|GetHUD))
  (Rendering|Components|TextRender|SetText (Variables|/Game/UI/WB_HUD.WB_HUD_C|GetXpText _hud) (Utilities|Text|FormatText "{Current} / {Needed}" (Utilities|Text|ToText(Integer) (Variables|Default|GetCurrentExp) false false) (Utilities|Text|ToText(Integer) (Variables|Default|GetExpForNextLevel) false false)))
  (Progress|SetPercent (Variables|/Game/UI/WB_HUD.WB_HUD_C|GetXpBar _hud) (/ (Variables|Default|GetCurrentExp) (Variables|Default|GetExpForNextLevel)))
  (return))

(fn UpdateLevel
  (Rendering|Components|TextRender|SetText (Variables|/Game/UI/WB_HUD.WB_HUD_C|GetLevelText (Variables|Default|GetHUD)) (Utilities|Text|ToText(Integer) (Variables|Default|GetCurrentLevel) false false))
  (return))

(fn AddExpPoints
  (params (Amount :type Integer))
  (Variables|Default|SetCurrentExp (+ Amount (Variables|Default|GetCurrentExp)))
  (if (>= (Variables|Default|GetCurrentExp) (Variables|Default|GetExpForNextLevel)) :!label _label
    (CallFunction|OnLevelUp)
    (goto _label)
    (else
      (ExpSystem|UpdateExp)
      (return))))

(fn InteractionTrace
  (bind _returnvalue (Transformation|GetActorLocation))
  (bind (_outhit _returnvalue_2) (Collision|SphereTraceByChannel _returnvalue (+ _returnvalue (* (Transformation|GetActorForwardVector) 1.6e+02)) 5e+01 "TraceTypeQuery1" false (Utilities|Array|MakeArray (Components|GetOwner)) "None"))
  (if _returnvalue_2
    (if (Utilities|DoesObjectImplementInterface (.HitActor (Collision|BreakHitResult _outhit)) "/Game/QuestSystem/Interface/BPI_Interact.BPI_Interact_C")
      (bind _output_get (Variables|Default|SetLookAtActor (.HitActor (Collision|BreakHitResult _outhit))))
      (Class|BPIInteract|Lookat(Message) _output_get)
      (else
        (Variables|Default|SetLookAtActor 0)))
    (else
      (Variables|Default|SetLookAtActor 0))))

(fn Interactwith
  (return ""))