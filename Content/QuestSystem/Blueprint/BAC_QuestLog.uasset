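; Quest log component that records active and completed quests by ID and handles turn-in.
; Each added quest spawns a BP_QuestBase actor, kept in an array and looked up by QuestID for state and completion.
; Turn-in awards the current stage's XP to the main player, shows a mission-complete widget, then marks the quest completed and notifies via CallOnQuestCompleted.
; A single tracker widget is created on first use and updated afterwards.
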(event EventBeginPlay)

(event EventTick
  (params (DeltaSeconds :type Float%20%28single-precision%29)))

(fn AddNewQuest
  (params (QuestID :type Name))
  (Utilities|Array|AddUnique (Variables|Default|GetCurrentActiveQuest) QuestID)
  (bind _returnvalue (Game|SpawnActorfromClass "/Game/QuestSystem/Blueprint/BP_QuestBase.BP_QuestBase_C" (Math|Transform|MakeTransform "0, 0, 0" "0, 0, 0" "1.000000,1.000000,1.000000") "AlwaysSpawn" "MultiplyWithRoot" 0 QuestID 0))
  (Utilities|Array|Add (Variables|Default|GetCurrentQuest) _returnvalue)
  (return _returnvalue))

(fn CompleteQuest
  (params (QuestID :type Name%20%28by%20ref%29))
  (Utilities|Array|AddUnique (Variables|Default|GetCompletedQuest) QuestID)
  (Utilities|Array|RemoveItem (Variables|Default|GetCurrentActiveQuest) QuestID)
  (bind _array_element (CallFunction|GetQuestActor QuestID))
  (Variables|/Game/QuestSystem/Blueprint/BP_QuestBase.BP_QuestBase_C|SetIsTurnedIn _array_element true)
  (Default|CallOnQuestCompleted _array_element)
  (UserInterface|CreateWidget "/Game/UI/Menu/W_MissionComplete.W_MissionComplete_C"))

(fn QuerryActiveQuest
  (params (QuestID :type Name))
  (return (Utilities|Array|ContainsItem (Variables|Default|GetCurrentActiveQuest) QuestID)))

(fn TrackQuest
  (params (QuestActor :type BP%20Quest%20Base%20Object%20Reference))
  (bind _tracker (Variables|Default|GetTracker)
    (:then
      (Default|Update _tracker QuestActor))
    (:else
      (bind _returnvalue (UserInterface|CreateWidget "/Game/QuestSystem/Widgets/W_QuestTracker.W_QuestTracker_C" 0 QuestActor))
      (bind _output_get (Variables|Default|SetTracker _returnvalue))
      (UserInterface|Viewport|AddtoViewport _output_get -1))))

(fn GetQuestActor
  (params (QuestId :type Name))
  (for _array_element (Variables|Default|GetCurrentQuest)
    (if (== (Variables|/Game/QuestSystem/Blueprint/BP_QuestBase.BP_QuestBase_C|GetQuestID _array_element) QuestId)
      (return _array_element))))

(fn TurninQuest
  (params (QuestId :type Name))
  (Utilities|FlowControl|Sequence
    (:then_0
      (bind _array_element (CallFunction|GetQuestActor QuestId))
      (Default|AddExpPoints (CallFunction|GetMainPlayer) (.XpReward (Utilities|Struct|BreakF_StageDetails (Variables|/Game/QuestSystem/Blueprint/BP_QuestBase.BP_QuestBase_C|GetCurrentStageDetails _array_element))))
      (bind _returnvalue (UserInterface|CreateWidget "/Game/UI/Menu/W_MissionComplete.W_MissionComplete_C"))
      (UserInterface|Viewport|AddtoViewport _returnvalue 0))
    (:then_1
      (CallFunction|CompleteQuest QuestId))))

(fn QuerryCompleted
  (params (QuestID :type Name))
  (bind _completedquest (Variables|Default|GetCompletedQuest))
  (bind _returnvalue (Utilities|Array|ContainsItem _completedquest QuestID))
  (bind _array_element (CallFunction|GetQuestActor QuestID))
  (Utilities|IsValid _array_element
    (:Is%20Valid
      (return _returnvalue (Variables|/Game/QuestSystem/Blueprint/BP_QuestBase.BP_QuestBase_C|GetIsTurnedIn _array_element)))
    (:Is%20Not%20Valid
      (return _returnvalue true))))