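; Actor component that makes its owner a quest giver, offering and rewarding the quest referenced by its QuestData row handle.
; InteractWith checks the player's BAC_QuestLog: a new quest is either auto-accepted into the log or shown in W_QuestGiver, based on its data table row.
; A completed but not yet turned-in quest opens W_QuestRewards instead.
; Each handled interaction returns the owner's display name.
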(event EventBeginPlay)

(event EventTick
  (params (DeltaSeconds :type Float%20%28single-precision%29)))

(fn DisplayQuest
  (bind _questdata (Variables|Default|GetQuestData))
  (bind _returnvalue (Utilities|GetDataTableRow (.datatable _questdata) (.rowname _questdata))
    (:then
      (bind _returnvalue_2 (UserInterface|CreateWidget "/Game/QuestSystem/Widgets/W_QuestGiver.W_QuestGiver_C" 0 _returnvalue (.rowname _questdata)))
      (UserInterface|Viewport|AddtoViewport _returnvalue_2 0))))

(fn DisplayRewards
  (bind _questdata (Variables|Default|GetQuestData))
  (bind _returnvalue (Utilities|GetDataTableRow "/Game/QuestSystem/DataTables/DT_Quest.DT_Quest" (.rowname _questdata))
    (:then
      (bind _returnvalue_2 (UserInterface|CreateWidget "/Game/QuestSystem/Widgets/W_QuestRewards.W_QuestRewards_C" 0 _returnvalue (.rowname _questdata)))
      (UserInterface|Viewport|AddtoViewport _returnvalue_2 0))))

(fn Interactwith
  (bind _returnvalue (Components|GetOwner))
  (bind _mainplayercharacter (CallFunction|GetMainPlayer))
  (bind _returnvalue_2 (Game|GetPlayerCharacter 0))
  (bind _questdata (Variables|Default|GetQuestData))
  (bind _returnvalue_3 (Actor|GetComponentbyClass _returnvalue_2 "/Game/QuestSystem/Blueprint/BAC_QuestLog.BAC_QuestLog_C"))
  (bind _returnvalue_4 (Utilities|GetDisplayName _returnvalue))
  (bind _bac_questlog (Variables|/Game/Blueprints/Player/BP_Player.BP_Player_C|GetBAC_QuestLog _mainplayercharacter))
  (if (and (not (Default|QuerryActiveQuest _bac_questlog (.rowname _questdata))) (not (.ReturnValue (Default|QuerryCompleted _bac_questlog (.rowname _questdata)))))
    (bind _returnvalue_5 (Utilities|GetDataTableRow "/Game/QuestSystem/DataTables/DT_Quest.DT_Quest" (.rowname (Variables|Default|GetQuestData)))
      (:then
        (if (.AutoAccept (Utilities|Struct|BreakF_QuestDetails _returnvalue_5))
          (Utilities|IsValid _returnvalue_3
            (:Is%20Valid
              (Default|AddNewQuest _returnvalue_3 (.rowname (Variables|Default|GetQuestData)))
              (return (Utilities|GetDisplayName (Components|GetOwner)))))
          (else
            (CallFunction|DisplayQuest)
            (return _returnvalue_4)))))
    (else
      (bind _array_element (Default|GetQuestActor (Variables|/Game/Blueprints/Player/BP_Player.BP_Player_C|GetBAC_QuestLog (CallFunction|GetMainPlayer)) (.rowname (Variables|Default|GetQuestData))))
      (if (and (Variables|/Game/QuestSystem/Blueprint/BP_QuestBase.BP_QuestBase_C|GetIsCompleted _array_element) (not (Variables|/Game/QuestSystem/Blueprint/BP_QuestBase.BP_QuestBase_C|GetIsTurnedIn _array_element)))
        (CallFunction|DisplayRewards)
        (return _returnvalue_4)))))