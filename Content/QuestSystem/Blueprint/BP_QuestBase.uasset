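; Base quest Blueprint that tracks one quest's objective progress through its stages, loaded from DT_Quest by QuestID.
; It binds to the player's objective-ID event to update a progress map, seeding one objective type from inventory on BeginPlay.
; Each completed objective shows a notification widget; a completed stage loads the next.
; After the last stage it marks the quest completed and, if AutoComplete is set, turns it in through BAC_QuestLog.
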(event EventBeginPlay
  (CallFunction|GetDetailsQuest)
  (EventDispatchers|BindEventtoOnObjectiveIdCalled (CallFunction|GetMainPlayer) (EventDispatchers|CreateEvent :!event OnObectiveIdHeard))
  (for _array_element (.Objectives (Utilities|Struct|BreakF_StageDetails (Variables|Default|GetCurrentStageDetails)))
    (if (Utilities|Enum|Equal(Enum) (.Type (Utilities|Struct|BreakF_ObjectiveDetails _array_element)) "NewEnumerator3")
      (bind _value (Default|QuerryInventory (Variables|/Game/Blueprints/Player/BP_Player.BP_Player_C|GetBAC_Inventory (CallFunction|GetMainPlayer)) (Utilities|String|StringToName (.ObjectiveID (Utilities|Struct|BreakF_ObjectiveDetails _array_element)))))
      (CallFunction|OnObectiveIdHeard (.ObjectiveID (Utilities|Struct|BreakF_ObjectiveDetails _array_element)) _value)))
  (Utilities|FlowControl|Delay 0.5)
  (bind _questcompleted (CallFunction|IsAllObjectiveComplete?))
  (Variables|Default|SetIsCompleted _questcompleted))

(fn ConstructionScript)

(fn OnObectiveIdHeard
  (params (ObjectiveId :type String) (Value :type Integer))
  (bind _currentobjectiveprogress (Variables|Default|GetCurrentObjectiveProgress))
  (bind (_value _returnvalue) (Utilities|Map|Find _currentobjectiveprogress ObjectiveId))
  (if (> (Class|KismetMathLibrary|SignOfInteger Value) 0)
    (if _returnvalue
      (if (< _value (.Quantity (Utilities|Struct|BreakF_ObjectiveDetails (CallFunction|GetObjectiveDatabyId ObjectiveId))))
        (Utilities|Map|Add (Variables|Default|GetCurrentObjectiveProgress) ObjectiveId (+ _value Value))
        (CallFunction|IsObjectiveComplete ObjectiveId)
        (Default|CallOnObjectiveHeard)
        (return))
      (else
        (return)))
    (else
      (Utilities|Map|Add (Variables|Default|GetCurrentObjectiveProgress) ObjectiveId (+ (.Value (Utilities|Map|Find (Variables|Default|GetCurrentObjectiveProgress) ObjectiveId)) Value))
      (return))))

(fn GetDetailsQuest
  (bind _returnvalue (Utilities|GetDataTableRow "/Game/QuestSystem/DataTables/DT_Quest.DT_Quest" (Variables|Default|GetQuestID))
    (:then
      (bind _output_get (Variables|Default|SetQuestDetails _returnvalue))
      (bind _output_get_2 (Variables|Default|SetCurrentStageDetails (Utilities|Array|Get(acopy) (.Stages (Utilities|Struct|BreakF_QuestDetails _output_get)) (Variables|Default|GetCurrentStage))))
      (Utilities|Map|Clear (Variables|Default|GetCurrentObjectiveProgress))
      (for _array_element (.Objectives (Utilities|Struct|BreakF_StageDetails _output_get_2))
        (Utilities|Map|Add (Variables|Default|GetCurrentObjectiveProgress) (.ObjectiveID (Utilities|Struct|BreakF_ObjectiveDetails _array_element)) 0)))))

(fn GetObjectiveDatabyId
  (params (ObjectiveId :type String))
  (for _array_element (.Objectives (Utilities|Struct|BreakF_StageDetails (Variables|Default|GetCurrentStageDetails)))
    (if (Utilities|Enum|Equal(Enum) ObjectiveId (.ObjectiveID (Utilities|Struct|BreakF_ObjectiveDetails _array_element)))
      (return _array_element))))

(fn IsObjectiveComplete
  (params (ObjectiveId :type String))
  (bind _array_element (CallFunction|GetObjectiveDatabyId ObjectiveId))
  (bind (_objectivename _description _type _objectiveid _quantity) (Utilities|Struct|BreakF_ObjectiveDetails _array_element))
  (if (>= (.Value (Utilities|Map|Find (Variables|Default|GetCurrentObjectiveProgress) ObjectiveId)) _quantity)
    (bind _returnvalue (UserInterface|CreateWidget "/Game/QuestSystem/Widgets/W_QuestNotification.W_QuestNotification_C" 0 _objectivename))
    (UserInterface|Viewport|AddtoViewport _returnvalue 0)
    (bind _questcompleted (CallFunction|IsAllObjectiveComplete?))
    (if _questcompleted
      (bind _result (Math|Integer|IncrementInt (Variables|Default|GetCurrentStage))
        (:%20%20
          (if (Utilities|Array|IsValidIndex (.stages (Variables|Default|GetQuestDetails)) _result)
            (CallFunction|GetDetailsQuest)
            (else
              (Variables|Default|SetIsCompleted true)
              (if (.autocomplete (Variables|Default|GetQuestDetails))
                (Default|TurninQuest (Actor|GetComponentbyClass (Game|GetPlayerCharacter 0) "/Game/QuestSystem/Blueprint/BAC_QuestLog.BAC_QuestLog_C") (Variables|Default|GetQuestID))))))))))

(fn IsAllObjectiveComplete?
  (for _array_element (.Objectives (Utilities|Struct|BreakF_StageDetails (Variables|Default|GetCurrentStageDetails)))
    (if (not (>= (.Value (Utilities|Map|Find (Variables|Default|GetCurrentObjectiveProgress) (.ObjectiveID (Utilities|Struct|BreakF_ObjectiveDetails _array_element)))) (.Quantity (Utilities|Struct|BreakF_ObjectiveDetails (CallFunction|GetObjectiveDatabyId (.ObjectiveID (Utilities|Struct|BreakF_ObjectiveDetails _array_element)))))))
      (bind _output_get (LocalVariables|SetLocal_IsComplete false))
      (return _output_get)))
  (return (LocalVariables|GetLocal_IsComplete)))