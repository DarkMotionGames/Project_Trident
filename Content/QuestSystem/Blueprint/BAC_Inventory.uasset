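; Inventory component for the quest system that stores item quantities in a Content map keyed by item.
; AddToInventory adds to the stored count, then notifies BP_Player through CallOnObjectiveIdCalled, passing the item name as objective ID and the added quantity, so pickups can feed quest objectives.
; QuerryInventory returns the stored count for an item.
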(event EventBeginPlay)

(event EventTick
  (params (DeltaSeconds :type Float%20%28single-precision%29)))

(fn AddtoInventory
  (params (Item :type Name) (Quantity :type Integer))
  (Utilities|Map|Add (Variables|Default|GetContent) Item (+ Quantity (.Value (Utilities|Map|Find (Variables|Default|GetContent) Item))))
  (bind _asbp_player (Utilities|Casting|CastToBP_Player (Game|GetPlayerCharacter 0)))
  (Default|CallOnObjectiveIdCalled _asbp_player (Utilities|String|ToString(Name) Item) Quantity))

(fn QuerryInventory
  (params (ItemName :type Name))
  (return (.Value (Utilities|Map|Find (Variables|Default|GetContent) ItemName))))